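; BP_Character is a top-down character Blueprint that handles movement-state input and camera control.
; Right mouse switches to aim and C to walk, both returning to run on release, while the mouse wheel adjusts the boom length within clamped limits.
; The construction script applies boom lag, length and rotation from variables.
; Two separate F-key bindings trigger a world camera shake and a death montage, apparently for testing.
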(event Input|MouseEvents|MouseWheelAxis
  (params (AxisValue :type Float%20%28single-precision%29))
  (bind _cameraboom (Variables|Default|GetCameraBoom))
  (Variables|/Script/Engine.SpringArmComponent|SetTargetArmLength _cameraboom (Math|Float|Clamp(Float) (+ (* AxisValue (Variables|Camera|GetChangeArmLengthStep)) (Variables|/Script/Engine.SpringArmComponent|GetTargetArmLength _cameraboom)) (Variables|Camera|GetMinSpringLength) (Variables|Camera|GetMaxSpringLength))))

(event Input|KeyboardEvents|F
  (params (Key :type Key%20Structure :default "None"))
  (:Pressed
    (CallFunction|CameraShake)))

(event Input|MouseEvents|RightMouseButton
  (params (Key :type Key%20Structure :default "None"))
  (:Pressed
    (Class|TopDownShooterCharacter|ChangeMovementState "Aim_State"))
  (:Released
    (Class|TopDownShooterCharacter|ChangeMovementState "Run_State")))

(event Input|KeyboardEvents|F
  (params (Key :type Key%20Structure :default "None"))
  (:Pressed
    (Animation|PlayAnimMontage "/Game/Blueprints/Character/Mannequin/Animations/NewAnim/AM_NewDeath_1.AM_NewDeath_1" 1.0 "None")))

(event Input|KeyboardEvents|C
  (params (Key :type Key%20Structure :default "None"))
  (:Pressed
    (Class|TopDownShooterCharacter|ChangeMovementState "Walk_State"))
  (:Released
    (Class|TopDownShooterCharacter|ChangeMovementState "Run_State")))

(fn ConstructionScript
  (bind _cameraboom (Variables|Default|GetCameraBoom))
  (Variables|/Script/Engine.SpringArmComponent|SetCameraLagSpeed _cameraboom (Variables|Camera|GetLagSpeed))
  (Variables|/Script/Engine.SpringArmComponent|SetbEnableCameraLag _cameraboom (Variables|Camera|GetFlow))
  (Variables|/Script/Engine.SpringArmComponent|SetTargetArmLength _cameraboom (Variables|Camera|GetHeight))
  (Transformation|SetRelativeRotation _cameraboom (Variables|Camera|GetCameraRotation) false false))

(fn CameraShake
  (Camera|PlayWorldCameraShake "/Game/Blueprints/Game/BP_CameraShake.BP_CameraShake_C" (Transformation|GetWorldLocation (Variables|Default|GetTopDownCameraComponent)) 0.0 3e+01))